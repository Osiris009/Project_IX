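; Player controller for Project IX that bootstraps the UI once the loading screen deactivates.
; It creates the CommonUI-style primary layout widget, registers it with the IX UI subsystem, then pushes the press-any-key screen onto the frontend stack through a gameplay-tag soft class lookup.
; It also registers the IMC_PIX mapping context with Enhanced Input user settings.
; The Possess and IA_Tab events are empty.
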(event `PIXLoadingScreenInterface.OnLoadingScreenDeactivated`
  (`|ExecutionSequence`
    (:`then_0`
      (bind _returnvalue (`|CreateWidget` "/Game/ProjectIX/UI/Widget/WBP_CAW_PrimaryLayout.WBP_CAW_PrimaryLayout_C" self))
      (`UserWidget.AddToViewport` _returnvalue 0)
      (`IX_UISubsystem.RegisterCreatedPrimaryLayoutWidget` (subsystem `IX_UISubsystem`) _returnvalue)
      (`AsyncAction_PushSoftWidget.PushSoftWidget` self (`UIFunctionLibrary.GetUISoftWidgetClassByTag` (struct :`TagName` "IXUI.Widget.PressAnyKeyScreen")) (struct :`TagName` "IXUI.WidgetStack.Frontend")))
    (:`then_1`
      (`EnhancedInputUserSettings.RegisterInputMappingContext` (`EnhancedInputSubsystemInterface.GetUserSettings` (subsystem `EnhancedInputLocalPlayerSubsystem`)) "/Game/Input/IMC_PIX.IMC_PIX"))))

(event `self.ReceivePossess`
  (params (PossessedPawn :type "Pawn Object Reference")))

(event `EnhancedInput|/Game/ProjectIX/Inputs/IA_Tab`
  (params (ActionValue :type Boolean) (ElapsedSeconds :type "Float (double-precision)") (TriggeredSeconds :type "Float (double-precision)") (InputAction :type "InputAction Object Reference" :default "/Game/ProjectIX/Inputs/IA_Tab.IA_Tab")))

(fn `UserConstructionScript`)